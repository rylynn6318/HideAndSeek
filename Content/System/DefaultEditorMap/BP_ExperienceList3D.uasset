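; Actor for the default editor map that spawns a centered row of teleport portals, one per user-facing experience.
; On BeginPlay it async-loads primary assets and builds a list from hand-added extras, default experiences inserted at the front, and the rest only if ShowAllExperiences is set.
; It then spawns a BP_TeleportToUserFacingExperience for each entry, spaced by PortalSpacing along the actor's local X axis.
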(event `self.ReceiveBeginPlay`
  (`KismetArrayLibrary.Array_Clear` (`self.UserFacingExperienceList`))
  (`KismetArrayLibrary.Array_Append` (`self.UserFacingExperienceList`) (`self.AdditionalExperiencesToShow`))
  (bind _outprimaryassetidlist (`KismetSystemLibrary.GetPrimaryAssetIdList` "HSUserFacingExperienceDefinition"))
  (bind _loaded (`AsyncActionLoadPrimaryAssetList.AsyncLoadPrimaryAssetList` _outprimaryassetidlist (`|MakeArray`))
    (:`Completed`
      (for _array_element _loaded
        (bind _ashsuser_facing_experience_definition (cast `HSUserFacingExperienceDefinition` _array_element))
        ;[1 1 1] Insert default experiences at the front, add the rest at the end if we want to show all of them
        (if true
          (if (`HSUserFacingExperienceDefinition.bIsDefaultExperience` _ashsuser_facing_experience_definition)
            (`KismetArrayLibrary.Array_Insert` (`self.UserFacingExperienceList`) _ashsuser_facing_experience_definition)
            (else
              (if (`self.ShowAllExperiences`) :!label _label
                (`KismetArrayLibrary.Array_Add` (`self.UserFacingExperienceList`) _ashsuser_facing_experience_definition))))
          (else
            (goto _label))))
      (for (_array_element_2 _array_index) (`self.UserFacingExperienceList`)
        (bind _returnvalue (`|SpawnActorFromClass` "/Game/System/DefaultEditorMap/BP_TeleportToUserFacingExperience.BP_TeleportToUserFacingExperience_C" (`KismetMathLibrary.MakeTransform` (`KismetMathLibrary.TransformLocation` (`SceneComponent.K2_GetComponentToWorld` (`self.DefaultSceneRoot`)) (`KismetMathLibrary.MakeVector` (* (+ _array_index (* -0.5 (`KismetArrayLibrary.Array_Length` (`self.UserFacingExperienceList`))) 0.5) (`self.PortalSpacing`)))) (`self.K2_GetActorRotation`)) "Undefined" "OverrideRootScale" null _array_element_2 null))
        (`KismetArrayLibrary.Array_Add` (`self.ExperiencePortals`) _returnvalue)))))

(fn `UserConstructionScript`)