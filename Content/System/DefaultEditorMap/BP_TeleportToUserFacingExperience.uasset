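; Teleporter actor in the default editor map that loads a user-facing experience when a local player's pawn overlaps it.
; On begin play it hands the experience to its widget component's experience tile, then disables the widget's ticking after a short delay.
; On overlap it pushes a non-interactive spinner to the menu layer, then hosts an offline session through the Common Session subsystem using the experience's hosting request.
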(event `self.ReceiveBeginPlay`
  (`|ExecutionSequence`
    (:`then_0`
      (bind _asw_experience_tile (cast `/Game/UI/Menu/W_ExperienceTile` (`WidgetComponent.GetWidget` (`self.Widget`))))
      (`/Game/UI/Menu/W_ExperienceTile.SetUserFacingExperience` _asw_experience_tile (`self.UserFacingExperienceToLoad`))
      (`KismetSystemLibrary.Delay` 0.2)
      (`WidgetComponent.SetTickMode` (`self.Widget`) "Disabled"))))

(event `self.ReceiveActorBeginOverlap`
  (params (OtherActor :type "Actor Object Reference"))
  (bind `_as폰` (cast `Pawn` OtherActor))
  (bind _returnvalue (`Pawn.GetController` `_as폰`))
  (`/Engine/EditorBlueprintResources/StandardMacros.IsValid` _returnvalue
    (:`Is Valid`
      (if (`Controller.IsLocalPlayerController` _returnvalue)
        (`self.LoadIntoExperience` (cast `PlayerController` _returnvalue :!pure true))))))

(event `LoadIntoExperience`
  (params (ForPlayer :type "PlayerController Object Reference"))
  (`/Engine/EditorBlueprintResources/StandardMacros.IsValid` (`self.UserFacingExperienceToLoad`)
    (:`Is Valid`
      (`AsyncAction_PushContentToLayerForPlayer.PushContentToLayerForPlayer` ForPlayer "/Game/UI/Menu/Experiences/W_NonInteractiveSpinner.W_NonInteractiveSpinner_C" (struct :`TagName` "UI.Layer.Menu")
        (:`AfterPush`
          (bind _returnvalue (`HSUserFacingExperienceDefinition.CreateHostingRequest` (`self.UserFacingExperienceToLoad`)))
          (set `CommonSession_HostSessionRequest.OnlineMode` "Offline" _returnvalue)
          (`CommonSessionSubsystem.HostSession` (subsystem `CommonSessionSubsystem`) ForPlayer _returnvalue))))))

(fn `UserConstructionScript`)